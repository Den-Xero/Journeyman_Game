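; Player kart Blueprint that handles driving, steering and held-item use.
; MoveForward ramps Speed, applies timed boost and swaps to a reversing camera; Tick feeds Speed into movement input along an arrow and the engine's RPM parameter.
; MoveRight yaws the kart directly.
; Use_Item dispatches on HeldItem, set by Add_Item; only Mushroom boost and Green Shell and Banana placeholder projectiles work, each using Ammo, while other items are empty stubs.
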(event Custom|Add_Item
  (params (Item_Name :type Name))
  ;[1 1 1] Add Item Function - Dylan
  (bind _output_get (Variables|Default|SetHeld_Item Item_Name))
  (Development|PrintString (Utilities|String|ToString(Name) _output_get)))

(event Custom|Drive
  (Audio|Parameter|SetFloatParameter (Variables|Default|GetEngine) "RPM" (Math|Float|Absolute(Float) (Variables|Default|GetSpeed)) :!class /Script/Engine.AudioComponent))

(event EventTick
  (params (DeltaSeconds :type Float%20%28single-precision%29))
  ;[1 1 1] Update Movment if speed > 0 - Leon
  (CallFunction|Drive)
  (if (> (Variables|Default|GetSpeed) 0.0)
    ;[1 1 1] Reversing Check from speed update - Leon
    (if (Variables|Default|GetIs_Reversing)
      (bind _output_get (Variables|Default|SetScale_Value -1.0))
      ;[1 1 1] Forward and back movement - Dylan
      (Pawn|Input|AddMovementInput (* (Math|Vector|GetForwardVector (Variables|Default|GetArrow1)) (Variables|Default|GetSpeed)) _output_get false)
      (else
        (Pawn|Input|AddMovementInput (* (Math|Vector|GetForwardVector (Variables|Default|GetArrow1)) (Variables|Default|GetSpeed)) 1.0 false)))))

(event Input|ActionEvents|InputActionUse_Item
  (params (Key :type Key%20Structure))
  ;[1 1 1] Item Use Event - Leon
  (:Pressed
    (switch name (Variables|Default|GetHeld_Item)
      (:Meteor
        (CallFunction|Meteor))
      (:Catapult
        (CallFunction|Catapult))
      (:Rock_Mushroom
        (CallFunction|RockMushroom))
      (:Boomerang
        (CallFunction|Boomerang))
      (:Dino_Horn
        (CallFunction|DinoHorn))
      (:Club
        (CallFunction|Club))
      (:Lightning_Tome
        (CallFunction|LightningTome))
      (:Smoke_Bomb
        (CallFunction|SmokeBomb))
      (:Flamethrower
        (CallFunction|FlameThrower))
      (:Holo_Item
        (CallFunction|HoloItem))
      (:Helmet
        (CallFunction|Helmet))
      (:Red_Shell
        (CallFunction|RedShell))
      (:Green_Shell
        (CallFunction|GreenShell))
      (:Mushroom
        (CallFunction|Mushroom))
      (:Banana
        (CallFunction|Banana))
      (:Star
        (CallFunction|Star))
      (:Triple_Mushroom
        (CallFunction|TripleMushroom))
      (:Triple_Green_Shell
        (CallFunction|TripleGreenShell))
      (:Triple_Red_Shell
        (CallFunction|TripleRedShell))
      (:Triple_Banana
        (CallFunction|TripleBanana)))))

(event Input|AxisEvents|InputAxisMoveForward
  (params (AxisValue :type Float%20%28single-precision%29))
  (bind _camera (Variables|Default|GetCamera))
  (bind _reversing_camera (Variables|Default|GetReversing_Camera))
  ;[1 1 1] Slowing car if reversing - Leon
  (Utilities|FlowControl|Delay 0.015)
  (bind _output_get (Variables|Default|SetIs_Reversing (== AxisValue -1.0)))
  (if (== AxisValue 0.0)
    (if (> (Variables|Default|GetSpeed) 0.0)
      (Variables|Default|SetSpeed (- (Variables|Default|GetSpeed) 0.5)))
    (if (Variables|Default|GetIs_Reversing)
      (Components|Activation|SetActive _camera false false :!label _label)
      (Components|Activation|SetActive _reversing_camera true false)
      (else
        (Components|Activation|SetActive _camera true false :!label _label_2)
        (Components|Activation|SetActive _reversing_camera false false)))
    (elif _output_get
      (if (< (Variables|Default|GetSpeed) (Variables|Default|GetMax_Reverse_Speed))
        (Variables|Default|SetSpeed (+ (Variables|Default|GetSpeed) 1.0))
        (goto _label)
        (else
          (goto _label)))
      (elif (< (Variables|Default|GetSpeed) (Variables|Default|GetMax_Speed))
        (Variables|Default|SetSpeed (+ (Variables|Default|GetSpeed) 0.1))
        (goto _label_2)
        (else
          (goto _label_2)))))
  ;[1 1 1] Apply Boost from pads/items - Leon
  (if (> (Variables|Default|GetBoost) 0.0)
    (if (> (Variables|Default|GetBoost_Timer) 0)
      (if (< (Variables|Default|GetSpeed) (Variables|Default|GetMax_Boost_Speed))
        (Variables|Default|SetSpeed (+ (Variables|Default|GetSpeed) (Variables|Default|GetBoost))))
      (Math|Integer|DecrementInt (Variables|Default|GetBoost_Timer)
        (:%20%20
          _))))
  (Development|PrintString (Utilities|String|ToString(Float) (Variables|Default|GetSpeed))))

(event Input|AxisEvents|InputAxisMoveRight
  (params (AxisValue :type Float%20%28single-precision%29))
  (bind _kart (Variables|Default|GetKart))
  (bind _returnvalue (Transformation|GetWorldRotation _kart))
  ;[1 1 1] Turning left and right - Dylan
  (Transformation|SetWorldRotation _kart (Math|Rotator|MakeRotator (.roll _returnvalue) (.pitch _returnvalue) (+ (.yaw _returnvalue) (/ AxisValue (Variables|Default|GetSteer_Speed)))) false false))

(fn ConstructionScript)

(fn GreenShell
  ;[1 1 1] Green Shell base code need to change spawn actor when I add in the proper ones - Callum
  (if (> (Variables|Default|GetAmmo) 0)
    (Game|SpawnActorfromClass "/Game/Programmers/Blueprints/Base_Projectile_code.Base_Projectile_code_C" (Transformation|GetWorldTransform (Variables|Default|GetFront_Firing_Point)) "Undefined" 0 0)
    (bind _result (Math|Integer|DecrementInt (Variables|Default|GetAmmo))
      (:%20%20
        (Variables|Default|SetAmmo _result)))
    (else
      (Development|PrintString "Out of ammo"))))

(fn TestFunt
  (Development|PrintString "Hello"))

(fn Meteor)

(fn Catapult)

(fn RockMushroom)

(fn Boomerang)

(fn DinoHorn)

(fn Club)

(fn LightningTome)

(fn SmokeBomb)

(fn FlameThrower)

(fn HoloItem)

(fn Helmet)

(fn RedShell)

(fn Mushroom
  (if (> (Variables|Default|GetAmmo) 0)
    (Variables|Default|SetBoost (+ (Variables|Default|GetBoost) (LocalVariables|GetBoost_Amount_Mushroom)))
    (Variables|Default|SetBoost_Timer (+ (Variables|Default|GetBoost_Timer) (LocalVariables|GetBoost_Timer_Amount_Mushroom)))
    (bind _result (Math|Integer|DecrementInt (Variables|Default|GetAmmo))
      (:%20%20
        (Variables|Default|SetAmmo _result)))
    (else
      (Development|PrintString "Out of ammo"))))

(fn Banana
  ;[1 1 1] Banana base code need to change spawn actor when I add in the proper ones - Callum
  (if (> (Variables|Default|GetAmmo) 0)
    (Game|SpawnActorfromClass "/Game/Programmers/Blueprints/Base_Projectile_code.Base_Projectile_code_C" (Transformation|GetWorldTransform (Variables|Default|GetFront_Firing_Point)) "Undefined" 0 0)
    (bind _result (Math|Integer|DecrementInt (Variables|Default|GetAmmo))
      (:%20%20
        (Variables|Default|SetAmmo _result)))
    (else
      (Development|PrintString "Out of ammo"))))

(fn Star)

(fn TripleMushroom)

(fn TripleGreenShell)

(fn TripleRedShell)

(fn TripleBanana)