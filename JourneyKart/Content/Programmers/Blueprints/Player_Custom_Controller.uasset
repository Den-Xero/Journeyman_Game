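; Custom player controller for a kart racing game that tracks laps and handles kart respawning.
; Update_Lap increments the lap count and its display text until the race completes, then calls a lap time check and prints the text.
; Respawn_Kart spawns a new Test_Kart at the stored respawn location and possesses it.
; Setup, timer, goal and time check events and functions are empty stubs.
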(event Custom|Start_Game_Setup)

(event Custom|Finished)

(event Custom|Update_Lap
  ;[0 0.9523 1] Updates the lap, adds to current lap and checks for lap record - Callum
  (if (Variables|Misc|GetRace_Complete)
    _
    (else
      (bind _output_get (Variables|Value_Variables|SetLap_Num (+ (Variables|Value_Variables|GetLap_Num) 1)))
      (bind _output_get_2 (Variables|Text_Variables|SetCurrent_Lap_Text (Utilities|Text|ToText(Integer) _output_get)))))
  (CallFunction|LapTimeCheck)
  (Development|PrintText _output_get_2))

(event Custom|Respawn_Kart
  ;[0 0.9523 1] Very very basic respawn event - Callum
  (bind _returnvalue (Game|SpawnActorfromClass "/Game/Programmers/Kart/Kart_BP/Test_Kart.Test_Kart_C" (Variables|Misc|GetRespawn_Location) "Undefined" 0 0))
  (Pawn|Possess _returnvalue))

(event Custom|Start_Race_Time)

(event Custom|Stop_Race_Time)

(event Custom|Start_Lap_time)

(event Custom|Stop_Lap_Time)

(fn ConstructionScript)

(fn InitText)

(fn LapTimeCheck)

(fn RaceTimeCheck)

(fn UpdateGoals)