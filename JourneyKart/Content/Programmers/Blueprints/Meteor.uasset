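; Meteor is a kart-racing projectile that homes in on the race leader and explodes, like a red shell.
; After a launch delay it enables homing on the Test_Kart in position 1.
; When movement stops, it spawns an explosion, enables Box overlaps and resizes the box through a timeline, then destroys itself.
; Box overlaps add timeout to Kart_BP actors only; the Test_Kart cast leads nowhere.
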(event OnComponentBeginOverlap(Box)
  (params (OverlappedComponent :type Primitive%20Component%20Object%20Reference) (OtherActor :type Actor%20Object%20Reference) (OtherComp :type Primitive%20Component%20Object%20Reference) (OtherBodyIndex :type Integer) (bFromSweep :type Boolean) (SweepResult :type Hit%20Result%20Structure%20%28by%20ref%29))
  ;[0 0.9523 1] Puts karts in to timeout when hit. - Callum
  (bind _askart_bp (Utilities|Casting|CastToKart_BP OtherActor)
    (:then
      (Variables|/Game/Programmers/Kart/Kart_BP/Kart_BP.Kart_BP_C|SetTime_Out _askart_bp (+ (Variables|/Game/Programmers/Kart/Kart_BP/Kart_BP.Kart_BP_C|GetTime_Out _askart_bp) 5)))
    (:CastFailed
      (Utilities|Casting|CastToTest_Kart OtherActor))))

(event OnProjectileStop(ProjectileMovement)
  (params (ImpactResult :type Hit%20Result%20Structure%20%28by%20ref%29))
  (bind _box (Variables|Default|GetBox))
  ;[0 0.9523 1] When bomb hits something it will stop wait 1.5s then turn gen overlaps on then make the collision box bigger for 1s then destroy itself. - Callum
  (Effects|SpawnEmitteratLocation "/Game/Starter_Project_Stuff/StarterContent/Particles/P_Explosion.P_Explosion" (Transformation|GetWorldLocation (Variables|Default|GetSphere)) "0, 0, 0" "1.000000,1.000000,1.000000" false)
  (Variables|/Script/Engine.PrimitiveComponent|SetbGenerateOverlapEvents _box true)
  (bind _curve (Timeline|Exploion Play)
    (:Update
      (Components|Box|SetBoxExtent _box _curve true))
    (:Finished
      (Actor|DestroyActor))))

(event EventBeginPlay
  (bind _projectilemovement (Variables|Default|GetProjectileMovement))
  ;[0 0.9523 1] Makes red shell travel to enemy after a delay - Callum
  (Utilities|FlowControl|Delay 4.0)
  (Variables|/Script/Engine.ProjectileMovementComponent|SetbIsHomingProjectile _projectilemovement true)
  (Variables|/Script/Engine.ProjectileMovementComponent|SetHomingAccelerationMagnitude _projectilemovement 1e+04)
  (bind _outactors (Actor|GetAllActorsOfClass "/Game/Programmers/Kart/Kart_BP/Test_Kart.Test_Kart_C"))
  (for _array_element _outactors
    (if (== (Variables|/Game/Programmers/Kart/Kart_BP/Test_Kart.Test_Kart_C|GetPosition _array_element) 1)
      (Variables|/Script/Engine.ProjectileMovementComponent|SetHomingTargetComponent _projectilemovement (Variables|/Game/Programmers/Kart/Kart_BP/Test_Kart.Test_Kart_C|GetDefaultSceneRoot _array_element)))))

(fn ConstructionScript)