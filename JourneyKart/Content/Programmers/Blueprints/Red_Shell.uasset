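; Red shell projectile for the kart game that homes in on a kart and adds timeout to any kart it hits.
; After a short launch delay it enables ProjectileMovement homing on the capsule of the first Kart_BP returned by GetAllActorsOfClass, without filtering by owner or distance.
; It destroys itself on hitting a kart, bouncing after the bounce counter reaches MaxBounce, or when its lifetime delay ends.
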(event OnProjectileBounce(ProjectileMovement)
  (params (ImpactResult :type Hit%20Result%20Structure%20%28by%20ref%29) (ImpactVelocity :type Vector%20%28by%20ref%29 :default "0, 0, 0"))
  ;[0 0.9523 1] Will check if shell has hit max bounce if so kills shell if not adds one to the bounce counter
  (if (== (Variables|Default|GetMax_Bounce) (Variables|Default|GetBounce_Counter))
    ;[0 0.9523 1] Puts karts in to timeout when hit. - Callum
    (Actor|DestroyActor)
    (else
      (bind _result (Math|Integer|IncrementInt (Variables|Default|GetBounce_Counter))
        (:%20%20
          (Variables|Default|SetBounce_Counter _result))))))

(event Collision|EventHit
  (params (MyComp :type Primitive%20Component%20Object%20Reference) (Other :type Actor%20Object%20Reference) (OtherComp :type Primitive%20Component%20Object%20Reference) (bSelfMoved :type Boolean) (HitLocation :type Vector :default "0, 0, 0") (HitNormal :type Vector :default "0, 0, 0") (NormalImpulse :type Vector :default "0, 0, 0") (Hit :type Hit%20Result%20Structure%20%28by%20ref%29))
  ;[0 0.9523 1] Puts karts in to timeout when hit. - Callum
  (bind _askart_bp (Utilities|Casting|CastToKart_BP Other))
  (Variables|/Game/Programmers/Kart/Kart_BP/Kart_BP.Kart_BP_C|SetTime_Out _askart_bp (+ (Variables|/Game/Programmers/Kart/Kart_BP/Kart_BP.Kart_BP_C|GetTime_Out _askart_bp) 5))
  (Actor|DestroyActor))

(event EventBeginPlay
  (bind _projectilemovement (Variables|Default|GetProjectileMovement))
  ;[0 0.9523 1] Makes red shell travel to enemy after a delay - Callum
  (Utilities|FlowControl|Delay 0.5)
  (Variables|/Script/Engine.ProjectileMovementComponent|SetbIsHomingProjectile _projectilemovement true)
  (Variables|/Script/Engine.ProjectileMovementComponent|SetHomingAccelerationMagnitude _projectilemovement 3.5e+03)
  (bind _outactors (Actor|GetAllActorsOfClass "/Game/Programmers/Kart/Kart_BP/Kart_BP.Kart_BP_C"))
  (Variables|/Script/Engine.ProjectileMovementComponent|SetHomingTargetComponent _projectilemovement (Variables|/Script/Engine.Character|GetCapsuleComponent (Utilities|Array|Get(acopy) _outactors)))
  (Utilities|FlowControl|Delay 4.0)
  (Actor|DestroyActor))

(fn ConstructionScript)