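; Kart-race checkpoint that players pass through, reporting its number when cleared.
; When a Test_Kart leaves the box, the dot product of its velocity and the arrow's forward vector checks travel direction.
; If that is zero or negative (not moving along the arrow), it fires the CheckpointCleared dispatcher, hides its particles and disables overlap events, so it clears only once.
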(event OnComponentEndOverlap(Box)
  (params (OverlappedComponent :type Primitive%20Component%20Object%20Reference) (OtherActor :type Actor%20Object%20Reference) (OtherComp :type Primitive%20Component%20Object%20Reference) (OtherBodyIndex :type Integer))
  ;[0 0.9523 1] Checkpoints for player to pass through - Callum
  (bind _astest_kart (Utilities|Casting|CastToTest_Kart OtherActor))
  (if (not (> (Math|Vector|DotProduct (Transformation|GetVelocity _astest_kart) (Math|Rotator|GetRotationXVector (Transformation|GetWorldRotation (Variables|Default|GetArrow)))) 0.0))
    (Default|CallCheckpointCleared (Variables|Default|GetCheckpoint_Number))
    (Development|SetHiddeninGame (Variables|Default|GetParticleSystem) true false)
    (Variables|/Script/Engine.PrimitiveComponent|SetbGenerateOverlapEvents (Variables|Default|GetBox) false)))

(fn ConstructionScript)