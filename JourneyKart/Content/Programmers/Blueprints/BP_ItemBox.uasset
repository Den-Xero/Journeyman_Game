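; BP_ItemBox is a kart racer item box with a spinning cube that hands an item to any Test_Kart that overlaps it.
; On overlap, ItemBoxLoot selects the item, which is passed to the kart's AddItem, then the cube hides and its collision turns off.
; Tick rotates the cube and, while it is hidden, runs a five-second Delay before restoring visibility and query-only collision.
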(event OnComponentBeginOverlap(Item_Box_Collision)
  (params (OverlappedComponent :type Primitive%20Component%20Object%20Reference) (OtherActor :type Actor%20Object%20Reference) (OtherComp :type Primitive%20Component%20Object%20Reference) (OtherBodyIndex :type Integer) (bFromSweep :type Boolean) (SweepResult :type Hit%20Result%20Structure%20%28by%20ref%29))
  (bind _item_box_loot (Variables|Default|GetItem_Box_Loot))
  ;[1 0.151 0.151] Calling item selection functions and passing the selected item to the kart blueprint - Dylan
  (if (Variables|Default|GetVisibility)
    (bind _astest_kart (Utilities|Casting|CastToTest_Kart OtherActor))
    (Default|SelectItem _item_box_loot)
    (bind _output_get (Variables|Default|SetItem_Type (Variables|/Game/Programmers/Blueprints/Item_Box_Loot.Item_Box_Loot_C|GetItem_To_Pass _item_box_loot)))
    (Default|AddItem _astest_kart _output_get)
    (Rendering|SetVisibility (Variables|Default|GetCube) false false)
    (Collision|SetCollisionEnabled (Variables|Default|GetItem_Box_Collision) "NoCollision")
    (Variables|Default|SetVisibility false)))

(event EventTick
  (params (DeltaSeconds :type Float%20%28single-precision%29))
  (Utilities|FlowControl|Sequence
    (:then_0
      ;[1 0.151 0.151] Make cube rotate - Dylan
      (Variables|Default|SetDelta_Seconds DeltaSeconds)
      (Transformation|AddLocalRotation (Variables|Default|GetCube) (Math|Rotator|MakeRotator 0.0 0.0 (* (Variables|Default|GetRotate_Speed) (Variables|Default|GetDelta_Seconds))) false false))
    (:then_1
      ;[1 0.151 0.151] Calling item selection functions and passing the selected item to the kart blueprint - Dylan
      ;;[1 0.151 0.151] Sets visiblity and collisions - Dylan
      (if (not (Variables|Default|GetVisibility))
        (Utilities|FlowControl|Delay 5.0)
        (Rendering|SetVisibility (Variables|Default|GetCube) true false)
        (Collision|SetCollisionEnabled (Variables|Default|GetItem_Box_Collision) "QueryOnly")
        (Variables|Default|SetVisibility true)))))

(fn ConstructionScript)