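; Item box loot Blueprint that picks a random kart item weighted by the player's race position.
; Select_Item reads Position from player 0's Test_Kart and loads the matching weight map for first through seventh place.
; CalculateTotal sums the weights, then ChooseItem rolls within that total and subtracts weights until one item wins.
; The chosen item is stored in ItemToPass.
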(event Custom|Select_Item
  ;[1 0.151 0.151] Selects a random item using functions - Dylan
  (bind _astest_kart (Utilities|Casting|CastToTest_Kart (Game|Player|GetPlayerPawn 0)))
  (switch int (Variables|/Game/Programmers/Kart/Kart_BP/Test_Kart.Test_Kart_C|GetPosition _astest_kart)
    (:1
      (Variables|Default|SetCurrent_Map (Variables|Default|GetFirst_Place_Items)))
    (:2
      (Variables|Default|SetCurrent_Map (Variables|Default|GetSecond_Place_Items)))
    (:3
      (Variables|Default|SetCurrent_Map (Variables|Default|GetThird_Place_Items)))
    (:4
      (Variables|Default|SetCurrent_Map (Variables|Default|GetFourth_Place_Items)))
    (:5
      (Variables|Default|SetCurrent_Map (Variables|Default|GetFifth_Place_Items)))
    (:6
      (Variables|Default|SetCurrent_Map (Variables|Default|GetSixth_Place_Items)))
    (:7
      (Variables|Default|SetCurrent_Map (Variables|Default|GetSeventh_Place_Items))))
  (bind _total (CallFunction|CalculateTotal))
  (Variables|Default|SetValue_Sum _total)
  (bind _item (CallFunction|ChooseItem))
  (Variables|Default|SetItem_To_Pass _item))

(fn CalculateTotal
  ;[1 0.151 0.151] Calculating the running total of each instance of each item - Dylan
  (bind _values (Utilities|Map|Values (Variables|Default|GetCurrent_Map)))
  (for _array_element _values
    (LocalVariables|SetRunning_Total (+ (LocalVariables|GetRunning_Total) _array_element)))
  (return (LocalVariables|GetRunning_Total)))

(fn ChooseItem
  (bind _current_map (Variables|Default|GetCurrent_Map))
  ;[1 0.151 0.151] Chooses item based on random values - Dylan
  (LocalVariables|SetRandom_Value (Math|Random|RandomFloatinRange 0.0 (Variables|Default|GetValue_Sum)))
  (bind _keys (Utilities|Map|Keys _current_map))
  (for _array_element _keys
    (if (<= (LocalVariables|GetRandom_Value) (.Value (Utilities|Map|Find _current_map _array_element)))
      (return _array_element)
      (else
        (LocalVariables|SetRandom_Value (- (LocalVariables|GetRandom_Value) (.Value (Utilities|Map|Find _current_map _array_element))))))))