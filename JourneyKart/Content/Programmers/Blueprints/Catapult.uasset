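; Catapult is a bomb projectile that explodes after landing and puts karts caught in the blast into timeout.
; Gravity switches on shortly after spawn; when the projectile stops, it waits briefly, spawns an explosion effect and enables overlap events on its Box.
; A timeline resizes the Box as the blast area, then destroys the actor.
; Overlapping Kart_BP actors gain timeout, while the Test_Kart fallback cast has no effect.
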(event OnComponentBeginOverlap(Box)
  (params (OverlappedComponent :type Primitive%20Component%20Object%20Reference) (OtherActor :type Actor%20Object%20Reference) (OtherComp :type Primitive%20Component%20Object%20Reference) (OtherBodyIndex :type Integer) (bFromSweep :type Boolean) (SweepResult :type Hit%20Result%20Structure%20%28by%20ref%29))
  ;[0 0.9523 1] Puts karts in to timeout when hit. - Callum
  (bind _askart_bp (Utilities|Casting|CastToKart_BP OtherActor)
    (:then
      (Variables|/Game/Programmers/Kart/Kart_BP/Kart_BP.Kart_BP_C|SetTime_Out _askart_bp (+ (Variables|/Game/Programmers/Kart/Kart_BP/Kart_BP.Kart_BP_C|GetTime_Out _askart_bp) 5)))
    (:CastFailed
      (Utilities|Casting|CastToTest_Kart OtherActor))))

(event OnProjectileStop(ProjectileMovement)
  (params (ImpactResult :type Hit%20Result%20Structure%20%28by%20ref%29))
  (bind _box (Variables|Default|GetBox))
  ;[0 0.9523 1] When bomb hits something it will stop wait 1.5s then turn gen overlaps on then make the collision box bigger for 1s then destroy itself. - Callum
  (Utilities|FlowControl|Delay 1.5)
  (Effects|SpawnEmitteratLocation "/Game/Starter_Project_Stuff/StarterContent/Particles/P_Explosion.P_Explosion" (Transformation|GetWorldLocation (Variables|Default|GetSphere)) "0, 0, 0" "2.500000,2.500000,2.500000" false)
  (Variables|/Script/Engine.PrimitiveComponent|SetbGenerateOverlapEvents _box true)
  (bind _curve (Timeline|Explosions Play)
    (:Update
      (Components|Box|SetBoxExtent _box _curve true))
    (:Finished
      (Actor|DestroyActor))))

(event EventBeginPlay
  ;[0 0.9523 1] Turns grav on after a delay then. - Callum
  (Utilities|FlowControl|Delay 0.5)
  (Variables|/Script/Engine.ProjectileMovementComponent|SetProjectileGravityScale (Variables|Default|GetProjectileMovement) 0.5))

(fn ConstructionScript)