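; Boomerang projectile item that penalises karts it hits and returns to the player.
; Shortly after spawning it homes on the first Test_Kart found, and it self-destructs after a further delay.
; Hitting a Kart_BP adds timeout.
; Reaching a Test_Kart, or stopping after a short delay, runs destruction and an AddItem call that passes on the use count incremented through Set_Boomerang_Used.
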(event OnProjectileStop(ProjectileMovement)
  (params (ImpactResult :type Hit%20Result%20Structure%20%28by%20ref%29))
  ;[0 0.9523 1] When boomerang hits player or stops moving it will be removed from play - Callum
  (Utilities|FlowControl|Delay 0.5)
  (Actor|DestroyActor)
  (Default|AddItem (stale Collision|EventHit _astest_kart) "Boomerang" (Variables|Default|GetBoomerang_used)))

(event Custom|Set_Boomerang_Used
  (params (Num :type Integer))
  ;[0 0.9523 1] Sets the number of times the item has used - Callum
  (bind _result (Math|Integer|IncrementInt Num)
    (:%20%20
      (Variables|Default|SetBoomerang_used _result))))

(event Collision|EventHit
  (params (MyComp :type Primitive%20Component%20Object%20Reference) (Other :type Actor%20Object%20Reference) (OtherComp :type Primitive%20Component%20Object%20Reference) (bSelfMoved :type Boolean) (HitLocation :type Vector :default "0, 0, 0") (HitNormal :type Vector :default "0, 0, 0") (NormalImpulse :type Vector :default "0, 0, 0") (Hit :type Hit%20Result%20Structure%20%28by%20ref%29))
  ;[0 0.9523 1] Puts karts in to timeout when hit. - Callum
  (bind _askart_bp (Utilities|Casting|CastToKart_BP Other)
    (:then
      (Variables|/Game/Programmers/Kart/Kart_BP/Kart_BP.Kart_BP_C|SetTime_Out _askart_bp (+ (Variables|/Game/Programmers/Kart/Kart_BP/Kart_BP.Kart_BP_C|GetTime_Out _askart_bp) 5)))
    (:CastFailed
      ;[0 0.9523 1] When boomerang hits player or stops moving it will be removed from play - Callum
      (bind _astest_kart (Utilities|Casting|CastToTest_Kart Other))
      (Actor|DestroyActor)
      (Default|AddItem _astest_kart "Boomerang" (Variables|Default|GetBoomerang_used)))))

(event EventBeginPlay
  (bind _projectilemovement (Variables|Default|GetProjectileMovement))
  ;[0 0.9523 1] Makes boomerang travel back to player after a delay - Callum
  (Utilities|FlowControl|Delay 0.5)
  (Variables|/Script/Engine.ProjectileMovementComponent|SetbIsHomingProjectile _projectilemovement true)
  (Variables|/Script/Engine.ProjectileMovementComponent|SetHomingAccelerationMagnitude _projectilemovement 3.5e+03)
  (bind _outactors (Actor|GetAllActorsOfClass "/Game/Programmers/Kart/Kart_BP/Test_Kart.Test_Kart_C"))
  (Variables|/Script/Engine.ProjectileMovementComponent|SetHomingTargetComponent _projectilemovement (Variables|/Game/Programmers/Kart/Kart_BP/Test_Kart.Test_Kart_C|GetBox (Utilities|Array|Get(acopy) _outactors)))
  (Utilities|FlowControl|Delay 4.0)
  (Actor|DestroyActor))

(fn ConstructionScript)