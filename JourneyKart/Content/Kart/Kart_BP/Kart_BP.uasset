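; Kart_BP is a player-drivable kart pawn controlled through two input axes.
; MoveForward adds movement input along Arrow1's forward vector, scaled by Speed and the axis value.
; MoveRight rotates the Kart component's world yaw directly by the axis value divided by SteerSpeed, so higher values steer more slowly.
; Steering is not scaled by delta time, so turn rate depends on frame rate.
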(event Input|AxisEvents|InputAxisMoveForward
  (params (AxisValue :type Float%20%28single-precision%29))
  ;[1 1 1] Forward and back movement - Dylan
  (Pawn|Input|AddMovementInput (* (Math|Vector|GetForwardVector (Variables|Default|GetArrow1)) (Variables|Default|GetSpeed)) AxisValue false))

(event Input|AxisEvents|InputAxisMoveRight
  (params (AxisValue :type Float%20%28single-precision%29))
  (bind _kart (Variables|Default|GetKart))
  (bind _returnvalue (Transformation|GetWorldRotation _kart))
  ;[1 1 1] Turning left and right - Dylan
  (Transformation|SetWorldRotation _kart (Math|Rotator|MakeRotator (.roll _returnvalue) (.pitch _returnvalue) (+ (.yaw _returnvalue) (/ AxisValue (Variables|Default|GetSteer_Speed)))) false false))

(fn ConstructionScript)