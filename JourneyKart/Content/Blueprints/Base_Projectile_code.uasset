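; Base projectile for a kart game, a bouncing shell that puts karts it hits into timeout.
; Hitting a Kart_BP adds to that kart's TimeOut and destroys the projectile, while other hit actors are ignored.
; Each ProjectileMovement bounce raises BounceCounter, and a bounce that occurs once the counter equals MaxBounce destroys the shell.
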(event OnProjectileBounce(ProjectileMovement)
  (params (ImpactResult :type Hit%20Result%20Structure%20%28by%20ref%29) (ImpactVelocity :type Vector%20%28by%20ref%29 :default "0, 0, 0"))
  ;[1 1 1] Will check if shell has hit max bounce if so kills shell if not adds one to the bounce counter
  (if (== (Variables|Default|GetMax_Bounce) (Variables|Default|GetBounce_Counter))
    ;[1 1 1] Puts karts in to timeout when hit. - Callum
    (Actor|DestroyActor)
    (else
      (bind _result (Math|Integer|IncrementInt (Variables|Default|GetBounce_Counter))
        (:%20%20
          (Variables|Default|SetBounce_Counter _result))))))

(event Collision|EventHit
  (params (MyComp :type Primitive%20Component%20Object%20Reference) (Other :type Actor%20Object%20Reference) (OtherComp :type Primitive%20Component%20Object%20Reference) (bSelfMoved :type Boolean) (HitLocation :type Vector :default "0, 0, 0") (HitNormal :type Vector :default "0, 0, 0") (NormalImpulse :type Vector :default "0, 0, 0") (Hit :type Hit%20Result%20Structure%20%28by%20ref%29))
  ;[1 1 1] Puts karts in to timeout when hit. - Callum
  (bind _askart_bp (Utilities|Casting|CastToKart_BP Other))
  (Variables|/Game/Kart/Kart_BP/Kart_BP.Kart_BP_C|SetTime_Out _askart_bp (+ (Variables|/Game/Kart/Kart_BP/Kart_BP.Kart_BP_C|GetTime_Out _askart_bp) 5))
  (Actor|DestroyActor))

(fn ConstructionScript)