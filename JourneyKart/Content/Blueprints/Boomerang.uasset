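; Boomerang projectile for the kart game that spins out karts it hits and homes back to the kart that threw it.
; After short delays it enables overlaps, then homes on the kart whose index matches ShootTracker, with a timed self-destroy.
; Overlapping the thrower destroys it and re-adds the Boomerang item with an incremented use count.
; A projectile stop runs the same destroy-and-add path, using the last overlapped kart reference.
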(event OnProjectileStop(ProjectileMovement)
  (params (ImpactResult :type Hit%20Result%20Structure%20%28by%20ref%29))
  ;[0 0.9523 1] When boomerang hits player or stops moving it will be removed from play - Callum
  (Utilities|FlowControl|Delay 0.5)
  (Actor|DestroyActor)
  (Default|AddItem (stale OnComponentBeginOverlap(Box) _asmain_kart) "Boomerang" (Variables|Default|GetBoomerang_used)))

(event OnComponentBeginOverlap(Box)
  (params (OverlappedComponent :type Primitive%20Component%20Object%20Reference) (OtherActor :type Actor%20Object%20Reference) (OtherComp :type Primitive%20Component%20Object%20Reference) (OtherBodyIndex :type Integer) (bFromSweep :type Boolean) (SweepResult :type Hit%20Result%20Structure%20%28by%20ref%29))
  ;[0 0.9523 1] Puts karts in to timeout when hit. - Callum
  (bind _asmain_kart (Utilities|Casting|CastToMain_Kart OtherActor))
  (if (== (Variables|/Game/Kart/Kart_BP/Character_Karts/Main_Kart.Main_Kart_C|GetIndex_Number _asmain_kart) (Variables|Default|GetShoot_Tracker))
    ;[0 0.9523 1] When boomerang hits player or stops moving it will be removed from play - Callum
    (Actor|DestroyActor)
    (Default|AddItem _asmain_kart "Boomerang" (Variables|Default|GetBoomerang_used))
    (else
      (Default|SpinOut _asmain_kart 5.0))))

(event Custom|Set_Boomerang_Used
  (params (Num :type Integer))
  ;[0 0.9523 1] Sets the number of times the item has used - Callum
  (bind _result (Math|Integer|IncrementInt Num)
    (:%20%20
      (Variables|Default|SetBoomerang_used _result))))

(event EventBeginPlay
  (bind _projectilemovement (Variables|Default|GetProjectileMovement))
  ;[0 0.9523 1] Makes boomerang travel back to player after a delay - Callum
  (Utilities|FlowControl|Delay 0.1)
  (Variables|/Script/Engine.PrimitiveComponent|SetbGenerateOverlapEvents (Variables|Default|GetBox) true)
  (Utilities|FlowControl|Delay 0.4)
  (Variables|/Script/Engine.ProjectileMovementComponent|SetbIsHomingProjectile _projectilemovement true)
  (Variables|/Script/Engine.ProjectileMovementComponent|SetHomingAccelerationMagnitude _projectilemovement 3.5e+03)
  (bind _outactors (Actor|GetAllActorsOfClass "/Game/Kart/Kart_BP/Character_Karts/Main_Kart.Main_Kart_C"))
  (for _array_element _outactors
    (if (== (Variables|/Game/Kart/Kart_BP/Character_Karts/Main_Kart.Main_Kart_C|GetIndex_Number _array_element) (Variables|Default|GetShoot_Tracker))
      (Variables|/Script/Engine.ProjectileMovementComponent|SetHomingTargetComponent _projectilemovement (Variables|/Game/Kart/Kart_BP/Character_Karts/Main_Kart.Main_Kart_C|GetBox _array_element))
      (Utilities|FlowControl|Delay 4.0)
      (Actor|DestroyActor))))

(fn ConstructionScript)