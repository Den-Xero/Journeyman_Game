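; Tank hazard that drives once along a referenced spline and spins out any kart it touches.
; On BeginPlay a timeline, with play rate set from the Time variable, moves the Box along the spline's length, following its rotation with a yaw offset.
; Box overlaps call SpinOut on Main_Kart actors.
; When the timeline finishes, the tank destroys itself and clears the Spawned flag on the Tank_Spawner.
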(event OnComponentBeginOverlap(Box)
  (params (OverlappedComponent :type Primitive%20Component%20Object%20Reference) (OtherActor :type Actor%20Object%20Reference) (OtherComp :type Primitive%20Component%20Object%20Reference) (OtherBodyIndex :type Integer) (bFromSweep :type Boolean) (SweepResult :type Hit%20Result%20Structure%20%28by%20ref%29))
  ;[1 0.151 0.151] Spins out karts - Dylan
  (bind _asmain_kart (Utilities|Casting|CastToMain_Kart OtherActor))
  (Default|SpinOut _asmain_kart 1.0))

(event Custom|Move%20Tank
  (bind _box (Variables|Default|GetBox))
  (bind _splinereference (Variables|Default|GetSplineReference))
  (bind _spline (Variables|/Game/Blueprints/Tank_Hazard/TankSpline.TankSpline_C|GetSpline _splinereference))
  ;[1 0.151 0.151] Tank moves along spline - Dylan
  (Components|Timeline|SetPlayRate (Variables|Default|GetMoveTank) (/ 1.0 (Variables|Default|GetTime)))
  (bind _movevalue (Timeline|MoveTank PlayFromStart)
    (:Update
      (Transformation|SetWorldTransform _box (Math|Transform|MakeTransform (Spline|GetLocationatDistanceAlongSpline _spline (Math|Float|Lerp 0.0 (Spline|GetSplineLength (Variables|/Game/Blueprints/Tank_Hazard/TankSpline.TankSpline_C|GetSpline (Variables|Default|GetSplineReference))) _movevalue) "World") (Math|Rotator|MakeRotator (.roll (Spline|GetRotationatDistanceAlongSpline _spline (Math|Float|Lerp 0.0 (Spline|GetSplineLength (Variables|/Game/Blueprints/Tank_Hazard/TankSpline.TankSpline_C|GetSpline (Variables|Default|GetSplineReference))) _movevalue) "World")) (.pitch (Spline|GetRotationatDistanceAlongSpline _spline (Math|Float|Lerp 0.0 (Spline|GetSplineLength (Variables|/Game/Blueprints/Tank_Hazard/TankSpline.TankSpline_C|GetSpline (Variables|Default|GetSplineReference))) _movevalue) "World")) (+ (.yaw (Spline|GetRotationatDistanceAlongSpline _spline (Math|Float|Lerp 0.0 (Spline|GetSplineLength (Variables|/Game/Blueprints/Tank_Hazard/TankSpline.TankSpline_C|GetSpline (Variables|Default|GetSplineReference))) _movevalue) "World")) -9e+01)) (Transformation|GetWorldScale _box)) false false))
    (:Finished
      (Actor|DestroyActor)
      (bind _returnvalue (Actor|GetActorOfClass "/Game/Blueprints/Tank_Hazard/Tank_Spawner.Tank_Spawner_C"))
      (Variables|/Game/Blueprints/Tank_Hazard/Tank_Spawner.Tank_Spawner_C|SetSpawned _returnvalue false))))

(event EventBeginPlay
  ;[1 0.151 0.151] Moves tank - Dylan
  (CallFunction|MoveTank))

(fn ConstructionScript)