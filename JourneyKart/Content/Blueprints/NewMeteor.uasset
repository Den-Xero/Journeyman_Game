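; Homing meteor projectile for a kart game that seeks the kart flagged as MeteorTarget.
; On BeginPlay it finds that kart in the game mode's AllKarts list and homes its ProjectileMovement on the kart's skeletal mesh.
; Any kart overlapping the capsule spins out with an explosion effect.
; The meteor destroys itself only on hitting a flagged kart, whose flag it clears first.
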(event OnComponentBeginOverlap(Capsule)
  (params (OverlappedComponent :type Primitive%20Component%20Object%20Reference) (OtherActor :type Actor%20Object%20Reference) (OtherComp :type Primitive%20Component%20Object%20Reference) (OtherBodyIndex :type Integer) (bFromSweep :type Boolean) (SweepResult :type Hit%20Result%20Structure%20%28by%20ref%29))
  ;[1 0.151 0.151] Spawns explosion and spins out the kart it hits - Dylan
  (bind _asmain_kart (Utilities|Casting|CastToMain_Kart OtherActor))
  (Default|SpinOut _asmain_kart 0.5)
  (Effects|SpawnEmitteratLocation "/Game/StarterContent/Particles/P_Explosion.P_Explosion" (Transformation|GetWorldLocation (Variables|/Game/Kart/Kart_BP/Character_Karts/Main_Kart.Main_Kart_C|GetBox _asmain_kart)) "0, 0, 0" "5.000000,5.000000,5.000000")
  (if (Variables|/Game/Kart/Kart_BP/Character_Karts/Main_Kart.Main_Kart_C|GetMeteor_Target _asmain_kart)
    (Variables|/Game/Kart/Kart_BP/Character_Karts/Main_Kart.Main_Kart_C|SetMeteor_Target _asmain_kart false)
    (Actor|DestroyActor)))

(event Custom|Move_Towards
  (bind _projectilemovement (Variables|Default|GetProjectileMovement))
  ;[1 0.151 0.151] Sets target for the homing meteor - Dylan
  (bind _target (CallFunction|FindTarget))
  (Variables|/Script/Engine.ProjectileMovementComponent|SetHomingTargetComponent _projectilemovement _target)
  (Variables|/Script/Engine.ProjectileMovementComponent|SetbIsHomingProjectile _projectilemovement true))

(event EventBeginPlay
  ;[1 0.151 0.151] Calls the custom event to start homing - Dylan
  (CallFunction|MoveTowards))

(fn ConstructionScript)

(fn FindTarget
  ;[1 0.151 0.151] Sets the homing target to the skeletal mesh component of the kart - Dylan
  (bind _asvehicle_game_mode (Utilities|Casting|CastToVehicleGameMode (Game|GetGameMode)))
  (for _array_element (Variables|/Game/VehicleBP/Blueprints/VehicleGameMode.VehicleGameMode_C|GetAll_Karts _asvehicle_game_mode)
    (if (Variables|/Game/Kart/Kart_BP/Character_Karts/Main_Kart.Main_Kart_C|GetMeteor_Target _array_element)
      (bind _output_get (Variables|Default|SetKart _array_element))
      (return (Actor|GetComponentbyClass _output_get "/Script/Engine.SkeletalMeshComponent")))))