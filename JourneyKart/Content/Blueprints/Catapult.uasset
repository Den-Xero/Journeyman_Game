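; Catapult projectile actor: a bomb that arcs forward, explodes when it stops and penalises karts caught in the blast.
; Tick moves it via the UpForwardArc macro, with upward movement switched off shortly after BeginPlay.
; When ProjectileMovement stops, it halts, spawns an explosion, enables box overlaps and resizes the box along a timeline before destroying itself.
; Box overlaps add timeout to Kart_BP; the Main_Kart cast leads to no action.
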(event OnComponentBeginOverlap(Box)
  (params (OverlappedComponent :type Primitive%20Component%20Object%20Reference) (OtherActor :type Actor%20Object%20Reference) (OtherComp :type Primitive%20Component%20Object%20Reference) (OtherBodyIndex :type Integer) (bFromSweep :type Boolean) (SweepResult :type Hit%20Result%20Structure%20%28by%20ref%29))
  ;[0 0.9523 1] Puts karts in to timeout when hit. - Callum
  (bind _askart_bp (Utilities|Casting|CastToKart_BP OtherActor)
    (:then
      (Variables|/Game/Kart/Kart_BP/Kart_BP.Kart_BP_C|SetTime_Out _askart_bp (+ (Variables|/Game/Kart/Kart_BP/Kart_BP.Kart_BP_C|GetTime_Out _askart_bp) 5)))
    (:CastFailed
      (Utilities|Casting|CastToMain_Kart OtherActor))))

(event OnProjectileStop(ProjectileMovement)
  (params (ImpactResult :type Hit%20Result%20Structure%20%28by%20ref%29))
  (bind _box (Variables|Default|GetBox))
  ;[0 0.9523 1] When bomb hits something it will stop wait 1.5s then turn gen overlaps on then make the collision box bigger for 1s then destroy itself. - Callum
  (Variables|Default|SetStop true)
  (Effects|SpawnEmitteratLocation "/Game/StarterContent/Particles/P_Explosion.P_Explosion" (Transformation|GetWorldLocation (Variables|Default|GetSphere)) "0, 0, 0" "2.500000,2.500000,2.500000" false)
  (Variables|/Script/Engine.PrimitiveComponent|SetbGenerateOverlapEvents _box true)
  (bind _curve (Timeline|Explosions Play)
    (:Update
      (Components|Box|SetBoxExtent _box _curve true))
    (:Finished
      (Actor|DestroyActor))))

(event EventBeginPlay
  ;[0 0.9523 1] Turns grav on after a delay. - Callum
  (Utilities|FlowControl|Delay 1.0)
  (Variables|Default|SetStop_Up_Movement true))

(event EventTick
  (params (DeltaSeconds :type Float%20%28single-precision%29))
  ;[0 0.9523 1] Movement with a Up arc. - Callum
  (bind (_pos_without_up _pos_with_up) (Utilities|UpForwardArc (Variables|Default|GetStop) (Variables|Default|GetMovement_Speed) (Variables|Default|GetUp_Movement) (Variables|Default|GetStop_Up_Movement) self)
    (:Out_Without_Up
      (Transformation|SetActorLocation _pos_without_up false false))
    (:Out_With_Up
      (Transformation|SetActorLocation _pos_with_up false false))))

(fn ConstructionScript)