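; Race tracker for a kart game that runs checkpoints, laps and finish through the player controller.
; On BeginPlay it passes lap and target times to the controller, numbers checkpoints and binds their cleared events.
; Each clear activates the next checkpoint and updates the respawn point, though CheckRaceComplete's logic is disconnected.
; Tick insertion-sorts karts by first-checkpoint distance to set positions only once, then prints a debug string.
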(event Custom|StartSequence
  (bind _checkpoints (Variables|Checkpoints|GetCheckpoints))
  ;[0 0.9523 1] Start sequence for chackpoint - Callum
  (for (_array_element _array_index) _checkpoints
    (Variables|/Game/Blueprints/Checkpoints.Checkpoints_C|SetCheckpoint_Number _array_element (+ _array_index 1))
    (Variables|Checkpoints|SetTotal_Checkpoints (Utilities|Array|Length _checkpoints))
    (CallFunction|ActivateNextCheckpoint (Utilities|Array|Get(acopy) _checkpoints))
    (for _array_element_2 _checkpoints
      (EventDispatchers|AssignCheckpointCleared _array_element_2 (delegate Custom|Checkpoint_Cleared)))))

(event Custom|Checkpoint_Cleared
  (params (Num_Checkpoint_cleared :type Integer))
  (bind _controller_reference (Variables|Default|GetController_Reference))
  ;[0 0.9523 1] When a checkpoint is cleared it check to see if on new lap and set next checkpoints up and ends game when race is completed - Callum
  (CallFunction|LapCheck Num_Checkpoint_cleared)
  (if (Variables|/Game/Blueprints/Player_Custom_Controller.Player_Custom_Controller_C|GetRace_Complete _controller_reference)
    (Default|Finished _controller_reference)))

(event Custom|Apply_Settings
  (bind _controller_reference (Variables|Default|GetController_Reference))
  ;[0 0.9523 1] Set up
  (Variables|/Game/Blueprints/Player_Custom_Controller.Player_Custom_Controller_C|SetMax_Laps _controller_reference (Variables|Laps|GetMax_Laps))
  (CallFunction|UpdateTimes)
  (Default|StartGameSetup _controller_reference))

(event EventTick
  (params (DeltaSeconds :type Float%20%28single-precision%29))
  (CallFunction|PosChecker)
  (Utilities|FlowControl|DoOnce false
    (:Completed
      (Variables|Default|SetDo_Not_Do true))))

(event EventBeginPlay
  ;[0 0.9523 1] Begin when game starts - Callum
  (bind _asplayer_custom_controller (Utilities|Casting|CastToPlayer_Custom_Controller (Game|GetPlayerController 0)))
  (bind _output_get (Variables|Default|SetController_Reference _asplayer_custom_controller))
  (CallFunction|ApplySettings)
  (CallFunction|StartSequence)
  (Default|StartRaceTime _output_get)
  (Default|StartLapTime _output_get))

(fn ConstructionScript)

(fn LapCheck
  (params (CheckPoint_Cleared :type Integer))
  ;[0 0.9523 1] Checks if lap is complete if so starts again if not activates next checkpoint, also checks if race is complete if not activates first checkpoint if, if race is complete can do that code when it is completed - Callum.
  (bind _output_get (LocalVariables|SetLocal_Checkpoint CheckPoint_Cleared))
  (if (== _output_get (Variables|Checkpoints|GetTotal_Checkpoints))
    (bind _is_race_complete (CallFunction|CheckRaceComplete))
    (if _is_race_complete
      _
      (else
        (CallFunction|ActivateNextCheckpoint (Utilities|Array|Get(acopy) (Variables|Checkpoints|GetCheckpoints)))))
    (else
      (CallFunction|ActivateNextCheckpoint (Utilities|Array|Get(acopy) (Variables|Checkpoints|GetCheckpoints) (LocalVariables|GetLocal_Checkpoint)))))
  ;[0 0.9523 1] Respawn kart at last checkpoint - Callum
  (Variables|/Game/Blueprints/Player_Custom_Controller.Player_Custom_Controller_C|SetRespawn_Location (Variables|Default|GetController_Reference) (Transformation|GetActorTransform (Utilities|Array|Get(acopy) (Variables|Checkpoints|GetCheckpoints) (- (LocalVariables|GetLocal_Checkpoint) 1)))))

(fn ActivateNextCheckpoint
  (params (Next_Checkpoint :type Checkpoints%20Object%20Reference))
  ;[0 0.9523 1] Makes next checkpoint work and make the particle system for the checkpoint seen in game - Callum
  (Development|SetHiddeninGame (Variables|/Game/Blueprints/Checkpoints.Checkpoints_C|GetParticleSystem Next_Checkpoint) false false)
  (Variables|/Script/Engine.PrimitiveComponent|SetbGenerateOverlapEvents (Variables|/Game/Blueprints/Checkpoints.Checkpoints_C|GetBox Next_Checkpoint) true))

(fn CheckRaceComplete
  ;[0 0.9523 1] Checks to see if lap is >= max lap if so says the race is completed if not says that the race is not completed - Callum
)

(fn UpdateTimes
  (bind _controller_reference (Variables|Default|GetController_Reference))
  ;[0 0.9523 1] Passing the tracker times to the controller times - Callum
  (Utilities|FlowControl|Sequence
    (:then_0
      (Variables|/Game/Blueprints/Player_Custom_Controller.Player_Custom_Controller_C|SetGold_Time _controller_reference (Variables|Laps|GetGold_Time)))
    (:then_1
      (Variables|/Game/Blueprints/Player_Custom_Controller.Player_Custom_Controller_C|SetSilver_Time _controller_reference (Variables|Laps|GetSilver_Time)))
    (:then_2
      (Variables|/Game/Blueprints/Player_Custom_Controller.Player_Custom_Controller_C|SetBronze_Time _controller_reference (Variables|Laps|GetBronze_Time)))
    (:then_3
      (Variables|/Game/Blueprints/Player_Custom_Controller.Player_Custom_Controller_C|SetBest_Lap_Time _controller_reference (Variables|Laps|GetBest_Lap_Time)))
    (:then_4
      (Variables|/Game/Blueprints/Player_Custom_Controller.Player_Custom_Controller_C|SetBest_Race_Time _controller_reference (Variables|Laps|GetWR_Time)))))

(fn PosChecker
  (bind _checkpoints (Variables|Checkpoints|GetCheckpoints))
  (bind _output (Utilities|Array|Get(acopy) _checkpoints))
  (bind _box (Variables|/Game/Blueprints/Checkpoints.Checkpoints_C|GetBox _output))
  (bind _returnvalue (Transformation|GetWorldLocation _box))
  (if (Variables|Default|GetDo_Not_Do)
    (Development|PrintString "Hello")
    (else
      (bind _outactors (Actor|GetAllActorsOfClass "/Game/Kart/Kart_BP/Character_Karts/Main_Kart.Main_Kart_C"))
      (bind _output_get (LocalVariables|SetKarts _outactors))
      (for (_array_element _array_index) _output_get
        (LocalVariables|SetCurrent_Target _array_element)
        (LocalVariables|SetCurrent_Target_Stepper _array_index)
        (LocalVariables|SetCurrent_Target_Distance (Math|Vector|Distance(Vector) (Transformation|GetWorldLocation (Variables|/Game/Kart/Kart_BP/Character_Karts/Main_Kart.Main_Kart_C|GetBox _array_element)) _returnvalue))
        (while (and (> (Math|Vector|Distance(Vector) (Transformation|GetWorldLocation (Variables|/Game/Kart/Kart_BP/Character_Karts/Main_Kart.Main_Kart_C|GetBox (Utilities|Array|Get(acopy) (LocalVariables|GetKarts) (- (LocalVariables|GetCurrent_Target_Stepper) 1)))) _returnvalue) (LocalVariables|GetCurrent_Target_Distance)) (> (LocalVariables|GetCurrent_Target_Stepper) 0))
          (Utilities|Array|Swap (LocalVariables|GetKarts) (LocalVariables|GetCurrent_Target_Stepper) (- (LocalVariables|GetCurrent_Target_Stepper) 1))
          (Math|Integer|DecrementInt (LocalVariables|GetCurrent_Target_Stepper)))
        (Utilities|Array|SetArrayElem (LocalVariables|GetKarts) (LocalVariables|GetCurrent_Target_Stepper) (LocalVariables|GetCurrent_Target)))
      (for (_array_element_2 _array_index_2) (LocalVariables|GetKarts)
        (Variables|/Game/Kart/Kart_BP/Character_Karts/Main_Kart.Main_Kart_C|SetPosition _array_element_2 (+ _array_index_2 1))))))