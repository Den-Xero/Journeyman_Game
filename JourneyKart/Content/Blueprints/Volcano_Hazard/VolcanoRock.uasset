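; VolcanoRock is a volcano hazard projectile that travels along a referenced spline and spins out any kart it hits.
; On BeginPlay, the MoveRock timeline plays at a rate set by Time, lerping distance along the spline to position the collision component.
; Overlapping a Main_Kart triggers SpinOut and destroys the rock.
; Reaching the spline's end spawns an explosion effect, then destroys it.
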(event OnComponentBeginOverlap(Rock_Collision)
  (params (OverlappedComponent :type Primitive%20Component%20Object%20Reference) (OtherActor :type Actor%20Object%20Reference) (OtherComp :type Primitive%20Component%20Object%20Reference) (OtherBodyIndex :type Integer) (bFromSweep :type Boolean) (SweepResult :type Hit%20Result%20Structure%20%28by%20ref%29))
  (bind _asmain_kart (Utilities|Casting|CastToMain_Kart OtherActor))
  (Default|SpinOut _asmain_kart 0.5)
  (Actor|DestroyActor))

(event Custom|ThrowRock
  (bind _rock_collision (Variables|Default|GetRock_Collision))
  (Components|Timeline|SetPlayRate (Variables|Default|GetMoveRock) (/ 1.0 (Variables|Default|GetTime)))
  (bind _movevalue (Timeline|MoveRock PlayFromStart)
    (:Update
      (Transformation|SetWorldTransform _rock_collision (Math|Transform|MakeTransform (Spline|GetLocationatDistanceAlongSpline (Variables|/Game/Blueprints/Volcano_Hazard/RockSpline.RockSpline_C|GetSpline (Variables|Default|GetSplineReference)) (Math|Float|Lerp 0.0 (Spline|GetSplineLength (Variables|/Game/Blueprints/Volcano_Hazard/RockSpline.RockSpline_C|GetSpline (Variables|Default|GetSplineReference))) _movevalue) "World") "0, 0, 0" (Transformation|GetWorldScale _rock_collision)) false false))
    (:Finished
      (Effects|SpawnEmitteratLocation "/Game/StarterContent/Particles/P_Explosion.P_Explosion" (Transformation|GetWorldLocation (Variables|Default|GetRock_Collision)) "0, 0, 0" "5.000000,5.000000,5.000000")
      (Actor|DestroyActor))))

(event EventBeginPlay
  (CallFunction|ThrowRock))

(fn ConstructionScript)