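; Red shell projectile that homes in on the kart one race position ahead of the shooter, wrapping toward the back for the leader.
; Start_Stuff caches the Route and target, flagging that kart for targeting UI.
; Tick steers along the Route spline, switching to VInterpTo homing when both actors' nearest spline points are close.
; Overlapping a kart clears the target flag, spins out that kart and destroys the shell.
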(event OnComponentBeginOverlap(r)
  (params (OverlappedComponent :type Primitive%20Component%20Object%20Reference) (OtherActor :type Actor%20Object%20Reference) (OtherComp :type Primitive%20Component%20Object%20Reference) (OtherBodyIndex :type Integer) (bFromSweep :type Boolean) (SweepResult :type Hit%20Result%20Structure%20%28by%20ref%29))
  ;[0 0.9523 1] Tells the kart to spinout when hit. - Callum
  (bind _asmain_kart (Utilities|Casting|CastToMain_Kart OtherActor))
  ;[1 0.6286 0] Disable Target UI on hit - Leon
  (Variables|/Game/Kart/Kart_BP/Character_Karts/Main_Kart.Main_Kart_C|SetCurrent_Red_Shell_Target? (stale Custom|Start_Stuff _asmain_kart) false)
  (Default|SpinOut _asmain_kart 0.5)
  (Actor|DestroyActor))

(event Custom|Start_Stuff
  (params (Pos :type Integer))
  ;[0 0.9523 1] Sets the spline that the read shell is meant to follow and the target as variables. - Callum
  (Variables|Default|SetShooters_Position Pos)
  (bind _returnvalue (Actor|GetActorOfClass "/Game/AI/Route.Route_C"))
  (Variables|Default|SetPath_To_Follow _returnvalue)
  (bind _outactors (Actor|GetAllActorsOfClass "/Game/Kart/Kart_BP/Character_Karts/Main_Kart.Main_Kart_C"))
  (for _array_element _outactors
    (if (== (Variables|/Game/Kart/Kart_BP/Character_Karts/Main_Kart.Main_Kart_C|GetPosition _array_element) (- (Variables|Default|GetShooters_Position) 1))
      (Variables|Default|SetTarget (Variables|/Game/Kart/Kart_BP/Character_Karts/Main_Kart.Main_Kart_C|GetBox _array_element) :!label _label)
      ;[1 0.6119 0] Set Target Variable for UI - Leon
      (bind _asmain_kart (Utilities|Casting|CastToMain_Kart _array_element))
      (Variables|/Game/Kart/Kart_BP/Character_Karts/Main_Kart.Main_Kart_C|SetCurrent_Red_Shell_Target? _asmain_kart true)
      (elif (== (- (Variables|Default|GetShooters_Position) 1) 0)
        (bind _output_get (Variables|Default|SetShooters_Position (Utilities|Array|Length _outactors)))
        (if (== _output_get (Variables|/Game/Kart/Kart_BP/Character_Karts/Main_Kart.Main_Kart_C|GetPosition _array_element))
          (goto _label))))))

(event EventTick
  (params (DeltaSeconds :type Float%20%28single-precision%29))
  (bind _path_to_follow (Variables|Default|GetPath_To_Follow))
  (bind _spline (Variables|/Game/AI/Route.Route_C|GetSpline _path_to_follow))
  ;[0 0.9523 1] Makes red shell travel to enemy after a delay - Callum
  (if (<= (Math|Vector|Distance(Vector) (Spline|FindLocationClosesttoWorldLocation _spline (Transformation|GetWorldLocation (Variables|Default|GetTarget)) "World") (Spline|FindLocationClosesttoWorldLocation _spline (Transformation|GetActorLocation) "World")) 5e+02)
    (Transformation|SetActorLocation (Math|Interpolation|VInterpTo (Transformation|GetActorLocation) (Transformation|GetWorldLocation (Variables|Default|GetTarget)) DeltaSeconds (/ (Variables|Default|GetMovement_Speed) 2.0)) false false)
    (else
      (Transformation|SetActorRotation (Math|Rotator|MakeRotator (.Roll (Math|Rotator|BreakRotator (Transformation|GetActorRotation))) (.Pitch (Math|Rotator|BreakRotator (Math|Rotator|MakeRotfromZX (Class|SplineComponent|FindUpVectorClosesttoWorldLocation (Variables|/Game/AI/Route.Route_C|GetSpline (Variables|Default|GetPath_To_Follow)) (Transformation|GetActorLocation) "World") (Transformation|GetActorForwardVector)))) (.Yaw (Math|Rotator|BreakRotator (Class|KismetMathLibrary|MakeRotfromYX (Class|SplineComponent|FindRightVectorClosesttoWorldLocation (Variables|/Game/AI/Route.Route_C|GetSpline (Variables|Default|GetPath_To_Follow)) (Transformation|GetActorLocation) "World") (Transformation|GetActorForwardVector))))))
      (Transformation|SetActorLocation (+ (Transformation|GetActorLocation) (* (Transformation|GetActorForwardVector) (Variables|Default|GetMovement_Speed))) false false))))

(fn ConstructionScript)