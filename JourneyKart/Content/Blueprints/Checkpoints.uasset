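; Race checkpoint actor that registers a Main_Kart passing through it.
; When a kart exits the box, a dot product of its velocity and the arrow's forward vector gates the clear, accepting only values of 0.1 or less.
; A clear broadcasts CheckpointCleared with the checkpoint number, stores that number on the kart, hides the particle system and disables the box's overlap events, making it single-use.
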(event OnComponentEndOverlap(Box)
  (params (OverlappedComponent :type Primitive%20Component%20Object%20Reference) (OtherActor :type Actor%20Object%20Reference) (OtherComp :type Primitive%20Component%20Object%20Reference) (OtherBodyIndex :type Integer))
  (bind _checkpoint_number (Variables|Default|GetCheckpoint_Number))
  ;[0 0.9523 1] Checkpoints for player to pass through - Callum
  (bind _asmain_kart (Utilities|Casting|CastToMain_Kart OtherActor))
  (if (not (> (Math|Vector|DotProduct (Transformation|GetVelocity _asmain_kart) (Math|Rotator|GetRotationXVector (Transformation|GetWorldRotation (Variables|Default|GetArrow)))) 0.1))
    (Default|CallCheckpointCleared _checkpoint_number)
    (Variables|/Game/Kart/Kart_BP/Character_Karts/Main_Kart.Main_Kart_C|SetCheckPoint_Num _asmain_kart _checkpoint_number)
    (Development|SetHiddeninGame (Variables|Default|GetParticleSystem) true false)
    (Variables|/Script/Engine.PrimitiveComponent|SetbGenerateOverlapEvents (Variables|Default|GetBox) false)))

(fn ConstructionScript)