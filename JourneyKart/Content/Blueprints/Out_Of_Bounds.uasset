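; Out-of-bounds trigger volume that respawns a Test_Kart entering its box.
; On overlap it sets a shared OOB flag and waits briefly, respawning the kart through its controller only if no kart exit has cleared the flag.
; After a respawn, EventInAction and disabled overlap events put the whole volume on a short cooldown before it re-arms.
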(event OnComponentBeginOverlap(Box)
  (params (OverlappedComponent :type Primitive%20Component%20Object%20Reference) (OtherActor :type Actor%20Object%20Reference) (OtherComp :type Primitive%20Component%20Object%20Reference) (OtherBodyIndex :type Integer) (bFromSweep :type Boolean) (SweepResult :type Hit%20Result%20Structure%20%28by%20ref%29))
  (bind _box (Variables|Default|GetBox))
  ;[0 0.9523 1] Makes kart respawn if out of bounds - Callum
  (if (not (Variables|Default|GetEvent_In_Action))
    (bind _astest_kart (Utilities|Casting|CastToTest_Kart OtherActor))
    (Variables|Default|SetOOB true)
    (Utilities|FlowControl|Delay 0.5)
    (if (Variables|Default|GetOOB)
      (Default|RespawnKart (Variables|/Game/Kart/Kart_BP/Test_Kart.Test_Kart_C|GetController_Reference _astest_kart) (Variables|/Game/Kart/Kart_BP/Test_Kart.Test_Kart_C|GetBox _astest_kart))
      (Variables|Default|SetEvent_In_Action true)
      (Variables|/Script/Engine.PrimitiveComponent|SetbGenerateOverlapEvents _box false)
      (Utilities|FlowControl|Delay 5.0)
      (Variables|Default|SetEvent_In_Action false)
      (Variables|/Script/Engine.PrimitiveComponent|SetbGenerateOverlapEvents _box true))))

(event OnComponentEndOverlap(Box)
  (params (OverlappedComponent :type Primitive%20Component%20Object%20Reference) (OtherActor :type Actor%20Object%20Reference) (OtherComp :type Primitive%20Component%20Object%20Reference) (OtherBodyIndex :type Integer))
  ;[0 0.9523 1] Makes kart respawn if out of bounds - Callum
  (Utilities|Casting|CastToTest_Kart OtherActor)
  (Variables|Default|SetOOB false))

(fn ConstructionScript)