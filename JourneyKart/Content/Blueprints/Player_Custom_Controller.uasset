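; Player controller for a Mario Kart-style racer that tracks laps and times and handles kart respawning.
; BeginPlay applies the GameInstance's selected character mesh to the possessed kart.
; Timelines drive race and lap clocks as text, and two nested timelines lift a respawning kart and ease it to the respawn transform.
; Lap updates increment the count until race completion, while time-check, setup and goal functions are empty stubs.
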(event Custom|Start_Game_Setup)

(event Custom|Finished)

(event Custom|Update_Lap
  ;[0 0.9523 1] Updates the lap, adds to current lap and checks for lap record - Callum
  (if (Variables|Misc|GetRace_Complete)
    _
    (else
      (bind _output_get (Variables|Value_Variables|SetLap_Num (+ (Variables|Value_Variables|GetLap_Num) 1)))
      (bind _output_get_2 (Variables|Text_Variables|SetCurrent_Lap_Text (Utilities|Text|ToText(Integer) _output_get)))))
  (CallFunction|LapTimeCheck)
  (Development|PrintText _output_get_2))

(event Custom|Respawn_Kart
  (params (Kart :type Box%20Component%20Object%20Reference%20%28by%20ref%29))
  (bind _returnvalue (Transformation|GetWorldTransform Kart))
  (bind _respawn_location (Variables|Misc|GetRespawn_Location))
  ;[0 0.9523 1] Respawn event working and looking good just end of it fuck and don't know y - Callum
  (Variables|Misc|SetTake_Control true)
  (bind _float_move1 (Timeline|Respawn_Move1 PlayFromStart)
    (:Update
      (Components|MoveComponentTo Kart (Math|Vector|Lerp(Vector) (.location _returnvalue) (+ "0, 0,500.000000" (.location _returnvalue)) _float_move1) (.rotation _returnvalue) true false 1.0 false)
      (bind _float_move2 (Timeline|Respawn_Move2 PlayFromStart)
        (:Update
          (Components|MoveComponentTo Kart (Math|Vector|Lerp(Vector) (.location _returnvalue) (+ (.location _respawn_location) "0, 0,120.000000") _float_move2) (Math|Rotator|Lerp(Rotator) (.rotation _returnvalue) (.rotation _respawn_location) _float_move2) true false 2.0 true))))))

(event Custom|Start_Race_Time
  ;[0 0.9523 1] Stars race timer and sets the timer as text in a format so it can be displayed to player on UI - Callum
  (bind _time (Timeline|Race_Time Play)
    (:Update
      (bind _output_get (Variables|Value_Variables|SetCurrent_Race_Time _time))
      (bind _output_get_2 (Variables|Text_Variables|SetCurrent_Race_Time_Text (Utilities|TimetoText _output_get)))
      (Development|PrintText _output_get_2 true true "(R=1.000000,G=0.000000,B=0.147162,A=1.000000)"))))

(event Custom|Stop_Race_Time
  ;[0 0.9523 1] Stars race timer and sets the timer as text in a format so it can be displayed to player on UI - Callum
  (bind _time (Timeline|Race_Time Stop)
    (:Update
      (bind _output_get (Variables|Value_Variables|SetCurrent_Race_Time _time))
      (bind _output_get_2 (Variables|Text_Variables|SetCurrent_Race_Time_Text (Utilities|TimetoText _output_get)))
      (Development|PrintText _output_get_2 true true "(R=1.000000,G=0.000000,B=0.147162,A=1.000000)"))))

(event Custom|Start_Lap_time
  ;[0 0.9523 1] Stars Lap timer and sets the timer as text in a format so it can be displayed to player on UI - Callum
  (bind _time (Timeline|Lap_Time PlayFromStart)
    (:Update
      (bind _output_get (Variables|Value_Variables|SetCurrent_Lap_Time _time))
      (bind _output_get_2 (Variables|Text_Variables|SetCurrent_Lap_Text (Utilities|TimetoText _output_get)))
      (Development|PrintText _output_get_2))))

(event Custom|Stop_Lap_Time
  ;[0 0.9523 1] Stars Lap timer and sets the timer as text in a format so it can be displayed to player on UI - Callum
  (bind _time (Timeline|Lap_Time Stop)
    (:Update
      (bind _output_get (Variables|Value_Variables|SetCurrent_Lap_Time _time))
      (bind _output_get_2 (Variables|Text_Variables|SetCurrent_Lap_Text (Utilities|TimetoText _output_get)))
      (Development|PrintText _output_get_2))))

(event EventBeginPlay
  (bind _askart_bp (Utilities|Casting|CastToKart_BP (Pawn|GetControlledPawn)))
  (bind _asmario_kart_game_instance (Utilities|Casting|CastToMarioKart_GameInstance (Game|GetGameInstance)))
  (Class|SkinnedMeshComponent|SetSkeletalMesh (Variables|/Script/Engine.Character|GetMesh _askart_bp) (Variables|/Game/MarioKart_GameInstance.MarioKart_GameInstance_C|GetSelectedCharacter _asmario_kart_game_instance) false))

(fn ConstructionScript)

(fn InitText)

(fn LapTimeCheck)

(fn RaceTimeCheck)

(fn UpdateGoals)