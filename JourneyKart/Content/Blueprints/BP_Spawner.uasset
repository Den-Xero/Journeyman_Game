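; BP_Spawner is a spawner actor that places a BP_ItemBox at its own transform on BeginPlay and stores it in CurrentObject.
; Tick polls that reference, printing a debug string while it is valid, and otherwise calls SpawnItem after a five-second Delay.
; SpawnItem does not update CurrentObject, so once the first box is gone, new boxes keep spawning on that delay.
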(event EventTick
  (params (DeltaSeconds :type Float%20%28single-precision%29))
  ;[1 1 1] Checking whether the item box has been picked up by the player - Dylan
  (Utilities|IsValid (Variables|Default|GetCurrent_Object)
    (:Is%20Valid
      (Development|PrintString "Item Already Spawned"))
    (:Is%20Not%20Valid
      (Utilities|FlowControl|Delay 5.0)
      (CallFunction|SpawnItem))))

(event EventBeginPlay
  ;[1 1 1] Spawns item box - Dylan
  (bind _returnvalue (Game|SpawnActorfromClass "/Game/Blueprints/BP_ItemBox.BP_ItemBox_C" (Transformation|GetActorTransform) "Undefined" 0 0))
  (Variables|Default|SetCurrent_Object _returnvalue))

(fn ConstructionScript)

(fn SpawnItem
  ;[1 1 1] Spawn function - Dylan
  (Game|SpawnActorfromClass "/Game/Blueprints/BP_ItemBox.BP_ItemBox_C" (Transformation|GetActorTransform) "Undefined" 0 0))