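; Coin pickup for a kart game that spins, adds to a kart's coin count and reappears after being collected.
; Overlapping a Main_Kart increments its CoinCount up to a cap of ten, hiding the coin and disabling sphere collision even at the cap.
; Tick rotates the sphere and, while hidden, uses a Delay to restore visibility and query collision five seconds later.
; An older, disconnected controller-based counting and destroy path remains unused.
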(event OnComponentBeginOverlap(Sphere)
  (params (OverlappedComponent :type Primitive%20Component%20Object%20Reference) (OtherActor :type Actor%20Object%20Reference) (OtherComp :type Primitive%20Component%20Object%20Reference) (OtherBodyIndex :type Integer) (bFromSweep :type Boolean) (SweepResult :type Hit%20Result%20Structure%20%28by%20ref%29))
  (bind _coin (Variables|Default|GetCoin))
  ;[1 0.151 0.151] Adds a coin to the total count of that kart - Dylan
  (bind _asmain_kart (Utilities|Casting|CastToMain_Kart OtherActor))
  (if (>= (Variables|/Game/Kart/Kart_BP/Character_Karts/Main_Kart.Main_Kart_C|GetCoin_Count _asmain_kart) 10)
    (Rendering|SetVisibility _coin false false)
    (Collision|SetCollisionEnabled (Variables|Default|GetSphere) "NoCollision")
    (Variables|Default|SetVisibility false)
    (else
      (Variables|/Game/Kart/Kart_BP/Character_Karts/Main_Kart.Main_Kart_C|SetCoin_Count _asmain_kart (+ (Variables|/Game/Kart/Kart_BP/Character_Karts/Main_Kart.Main_Kart_C|GetCoin_Count _asmain_kart) 1))
      (Rendering|SetVisibility _coin false false)
      (Collision|SetCollisionEnabled (Variables|Default|GetSphere) "NoCollision")
      (Variables|Default|SetVisibility false))))

(event EventTick
  (params (DeltaSeconds :type Float%20%28single-precision%29))
  ;[1 0.151 0.151] Adds rotation to the mesh and then checks visibility - Dylan
  (Utilities|FlowControl|Sequence
    (:then_0
      (Variables|Default|SetDelta_Seconds DeltaSeconds)
      (Transformation|AddLocalRotation (Variables|Default|GetSphere) (Math|Rotator|MakeRotator 0.0 0.0 (* (Variables|Default|GetRotate_Speed) (Variables|Default|GetDelta_Seconds))) false false))
    (:then_1
      (if (not (Variables|Default|GetVisibility))
        (Utilities|FlowControl|Delay 5.0)
        (Rendering|SetVisibility (Variables|Default|GetCoin) true false)
        (Collision|SetCollisionEnabled (Variables|Default|GetSphere) "QueryOnly")
        (Variables|Default|SetVisibility true)))))

(fn ConstructionScript)