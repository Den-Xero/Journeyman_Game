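; Red shell projectile that homes in on karts and spins out the one it hits.
; Every 0.2 seconds from BeginPlay, it searches all Main_Kart actors for the nearest one not flagged IsUser.
; That kart's BoxComponent becomes the ProjectileMovement homing target.
; When its sphere overlaps any Main_Kart, it calls SpinOut on that kart and destroys itself.
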(event OnComponentBeginOverlap(Sphere)
  (params (OverlappedComponent :type Primitive%20Component%20Object%20Reference) (OtherActor :type Actor%20Object%20Reference) (OtherComp :type Primitive%20Component%20Object%20Reference) (OtherBodyIndex :type Integer) (bFromSweep :type Boolean) (SweepResult :type Hit%20Result%20Structure%20%28by%20ref%29))
  (bind _asmain_kart (Utilities|Casting|CastToMain_Kart OtherActor))
  (Default|SpinOut _asmain_kart 0.5)
  (Actor|DestroyActor))

(event Custom|Move_Towards
  (bind _projectilemovement (Variables|Default|GetProjectileMovement))
  (bind _target (CallFunction|FindTarget))
  (Variables|/Script/Engine.ProjectileMovementComponent|SetHomingTargetComponent _projectilemovement _target)
  (Variables|/Script/Engine.ProjectileMovementComponent|SetbIsHomingProjectile _projectilemovement true))

(event EventBeginPlay
  (CallFunction|MoveTowards :!label _label)
  (Utilities|FlowControl|Delay 0.2)
  (goto _label))

(fn ConstructionScript)

(fn FindTarget
  (bind _outactors (Actor|GetAllActorsOfClass "/Game/Kart/Kart_BP/Character_Karts/Main_Kart.Main_Kart_C"))
  (for _array_element _outactors
    (if (not (Variables|/Game/Kart/Kart_BP/Character_Karts/Main_Kart.Main_Kart_C|GetIs_User _array_element))
      (if (< (Math|Vector|VectorLength (- (Transformation|GetActorLocation _array_element) (Transformation|GetActorLocation))) (Variables|Default|GetClosest))
        (Variables|Default|SetClosest (Math|Vector|VectorLength (- (Transformation|GetActorLocation _array_element) (Transformation|GetActorLocation))))
        (Variables|Default|SetTarget _array_element))))
  (return (Actor|GetComponentbyClass (Variables|Default|GetTarget) "/Script/Engine.BoxComponent")))