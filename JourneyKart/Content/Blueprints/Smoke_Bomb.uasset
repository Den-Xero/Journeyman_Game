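; Smoke bomb projectile for the kart game that is launched in an arc, then destroys itself when a Main_Kart overlaps its box.
; Tick moves it with the UpForwardArc helper; one second after BeginPlay the upward motion stops and box overlap events turn on.
; When ProjectileMovement stops, forward motion halts and the particle system appears after a short delay.
; The UI smoke screen and final particle effect are still TODO.
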(event OnProjectileStop(ProjectileMovement)
  (params (ImpactResult :type Hit%20Result%20Structure%20%28by%20ref%29))
  ;[0 0.9523 1] Turns particle system viz ingame after it lands. Need to add particle when it is ready. - Callum
  (Variables|Default|SetStop true)
  (Utilities|FlowControl|Delay 0.5)
  (Development|SetHiddeninGame (Variables|Default|GetParticleSystem) false false))

(event OnComponentBeginOverlap(Box)
  (params (OverlappedComponent :type Primitive%20Component%20Object%20Reference) (OtherActor :type Actor%20Object%20Reference) (OtherComp :type Primitive%20Component%20Object%20Reference) (OtherBodyIndex :type Integer) (bFromSweep :type Boolean) (SweepResult :type Hit%20Result%20Structure%20%28by%20ref%29))
  ;[0 0.9523 1] TODO adds smoke screen to ui when it is in place. - Callum
  (Utilities|Casting|CastToMain_Kart OtherActor)
  (Actor|DestroyActor))

(event EventBeginPlay
  ;[0 0.9523 1] Turns grav on after a delay then and lets the box gen overlap events. - Callum
  (Utilities|FlowControl|Delay 1.0)
  (Variables|Default|SetStop_Up_Movement true)
  (Variables|/Script/Engine.PrimitiveComponent|SetbGenerateOverlapEvents (Variables|Default|GetBox) true))

(event EventTick
  (params (DeltaSeconds :type Float%20%28single-precision%29))
  ;[0 0.9523 1] Movement with a Up arc. - Callum
  (bind (_pos_without_up _pos_with_up) (Utilities|UpForwardArc (Variables|Default|GetStop) (Variables|Default|GetMovement_Speed) (Variables|Default|GetUp_Movement) (Variables|Default|GetStop_Up_Movement) self)
    (:Out_Without_Up
      (Transformation|SetActorLocation _pos_without_up false false))
    (:Out_With_Up
      (Transformation|SetActorLocation _pos_with_up false false))))

(fn ConstructionScript)