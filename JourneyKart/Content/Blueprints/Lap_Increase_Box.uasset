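; Lap trigger box that counts a lap when the player's pawn overlaps it.
; On overlap by player 0's pawn, it calls UpdateLap on the Player_Custom_Controller.
; An AddedRecently flag with a 30-second delay blocks repeat counts from the same crossing.
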(event Collision|EventActorBeginOverlap
  (params (OtherActor :type Actor%20Object%20Reference))
  (if (not (Variables|Default|GetAdded%20Recently))
    (if (== OtherActor (Game|Player|GetPlayerPawn 0))
      (bind _asplayer_custom_controller (Utilities|Casting|CastToPlayer_Custom_Controller (Game|GetPlayerController 0)))
      (Default|UpdateLap _asplayer_custom_controller)
      (Variables|Default|SetAdded%20Recently true)
      (Utilities|FlowControl|Delay 3e+01)
      (Variables|Default|SetAdded%20Recently false))))

(fn ConstructionScript)