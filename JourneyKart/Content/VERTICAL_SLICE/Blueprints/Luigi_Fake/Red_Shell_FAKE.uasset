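; Fake red shell actor that travels along a spline path by itself once play begins.
; On BeginPlay it finds the Shell_Spline actor in the level and starts a timeline with its play rate derived from a Time variable.
; Each update places the Shell component at the matching distance along the spline, following its rotation with a yaw offset.
; It has no overlap or hit logic.
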(event Custom|Move%20Shell
  (bind _shell (Variables|Default|GetShell))
  ;[1 0.151 0.151] Tank moves along spline - Dylan
  (Components|Timeline|SetPlayRate (Variables|Default|GetMove_Shell) (/ 1.0 (Variables|Default|GetTime)))
  (bind _movevalue (Timeline|Move_Shell PlayFromStart)
    (:Update
      (Transformation|SetWorldTransform _shell (Math|Transform|MakeTransform (Spline|GetLocationatDistanceAlongSpline (Variables|/Game/VERTICAL_SLICE/Blueprints/Luigi_Fake/Shell_Spline.Shell_Spline_C|GetSpline (Variables|Default|GetSplineReference)) (Math|Float|Lerp 0.0 (Spline|GetSplineLength (Variables|/Game/VERTICAL_SLICE/Blueprints/Luigi_Fake/Shell_Spline.Shell_Spline_C|GetSpline (Variables|Default|GetSplineReference))) _movevalue) "World") (Math|Rotator|MakeRotator (.roll (Spline|GetRotationatDistanceAlongSpline (Variables|/Game/VERTICAL_SLICE/Blueprints/Luigi_Fake/Shell_Spline.Shell_Spline_C|GetSpline (Variables|Default|GetSplineReference)) (Math|Float|Lerp 0.0 (Spline|GetSplineLength (Variables|/Game/VERTICAL_SLICE/Blueprints/Luigi_Fake/Shell_Spline.Shell_Spline_C|GetSpline (Variables|Default|GetSplineReference))) _movevalue) "World")) (.pitch (Spline|GetRotationatDistanceAlongSpline (Variables|/Game/VERTICAL_SLICE/Blueprints/Luigi_Fake/Shell_Spline.Shell_Spline_C|GetSpline (Variables|Default|GetSplineReference)) (Math|Float|Lerp 0.0 (Spline|GetSplineLength (Variables|/Game/VERTICAL_SLICE/Blueprints/Luigi_Fake/Shell_Spline.Shell_Spline_C|GetSpline (Variables|Default|GetSplineReference))) _movevalue) "World")) (+ (.yaw (Spline|GetRotationatDistanceAlongSpline (Variables|/Game/VERTICAL_SLICE/Blueprints/Luigi_Fake/Shell_Spline.Shell_Spline_C|GetSpline (Variables|Default|GetSplineReference)) (Math|Float|Lerp 0.0 (Spline|GetSplineLength (Variables|/Game/VERTICAL_SLICE/Blueprints/Luigi_Fake/Shell_Spline.Shell_Spline_C|GetSpline (Variables|Default|GetSplineReference))) _movevalue) "World")) -9e+01)) (Transformation|GetWorldScale _shell)) false false))))

(event EventBeginPlay
  ;[1 0.151 0.151] Moves tank - Dylan
  (bind _returnvalue (Actor|GetActorOfClass "/Game/VERTICAL_SLICE/Blueprints/Luigi_Fake/Shell_Spline.Shell_Spline_C"))
  (Variables|Default|SetSplineReference _returnvalue)
  (CallFunction|MoveShell))

(event Collision|EventActorBeginOverlap
  (params (OtherActor :type Actor%20Object%20Reference)))

(event EventTick
  (params (DeltaSeconds :type Float%20%28single-precision%29)))

(fn ConstructionScript)