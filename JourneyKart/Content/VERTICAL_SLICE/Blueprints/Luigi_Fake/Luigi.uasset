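; Luigi is an actor, described as a tank, that travels along a level-placed spline and then fires a fake red shell.
; On BeginPlay it finds the Luigi_Spline actor and starts a timeline with play rate scaled by the inverse of its Time variable.
; Each update maps the timeline alpha to spline distance, setting the Box's world location and rotation.
; When the timeline finishes, it spawns Red_Shell_FAKE at FiringPoint.
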(event Custom|Move%20luigi
  (bind _box (Variables|Default|GetBox))
  ;[1 0.151 0.151] Tank moves along spline - Dylan
  (Components|Timeline|SetPlayRate (Variables|Default|GetMove_Luigi) (/ 1.0 (Variables|Default|GetTime)))
  (bind _movevalue (Timeline|Move_Luigi PlayFromStart)
    (:Update
      (Transformation|SetWorldTransform _box (Math|Transform|MakeTransform (Spline|GetLocationatDistanceAlongSpline (Variables|/Game/VERTICAL_SLICE/Blueprints/Luigi_Fake/Luigi_Spline.Luigi_Spline_C|GetSpline (Variables|Default|GetSplineReference)) (Math|Float|Lerp 0.0 (Spline|GetSplineLength (Variables|/Game/VERTICAL_SLICE/Blueprints/Luigi_Fake/Luigi_Spline.Luigi_Spline_C|GetSpline (Variables|Default|GetSplineReference))) _movevalue) "World") (Math|Rotator|MakeRotator (.roll (Spline|GetRotationatDistanceAlongSpline (Variables|/Game/VERTICAL_SLICE/Blueprints/Luigi_Fake/Luigi_Spline.Luigi_Spline_C|GetSpline (Variables|Default|GetSplineReference)) (Math|Float|Lerp 0.0 (Spline|GetSplineLength (Variables|/Game/VERTICAL_SLICE/Blueprints/Luigi_Fake/Luigi_Spline.Luigi_Spline_C|GetSpline (Variables|Default|GetSplineReference))) _movevalue) "World")) (.pitch (Spline|GetRotationatDistanceAlongSpline (Variables|/Game/VERTICAL_SLICE/Blueprints/Luigi_Fake/Luigi_Spline.Luigi_Spline_C|GetSpline (Variables|Default|GetSplineReference)) (Math|Float|Lerp 0.0 (Spline|GetSplineLength (Variables|/Game/VERTICAL_SLICE/Blueprints/Luigi_Fake/Luigi_Spline.Luigi_Spline_C|GetSpline (Variables|Default|GetSplineReference))) _movevalue) "World")) (.yaw (Spline|GetRotationatDistanceAlongSpline (Variables|/Game/VERTICAL_SLICE/Blueprints/Luigi_Fake/Luigi_Spline.Luigi_Spline_C|GetSpline (Variables|Default|GetSplineReference)) (Math|Float|Lerp 0.0 (Spline|GetSplineLength (Variables|/Game/VERTICAL_SLICE/Blueprints/Luigi_Fake/Luigi_Spline.Luigi_Spline_C|GetSpline (Variables|Default|GetSplineReference))) _movevalue) "World"))) (Transformation|GetWorldScale _box)) false false))
    (:Finished
      (Game|SpawnActorfromClass "/Game/VERTICAL_SLICE/Blueprints/Luigi_Fake/Red_Shell_FAKE.Red_Shell_FAKE_C" (Math|Conversions|ToTransform(Vector) (Transformation|GetWorldLocation (Variables|Default|GetFiring%20point))) "Undefined" 0 0 2.0 0))))

(event EventBeginPlay
  ;[1 0.151 0.151] Moves tank - Dylan
  (bind _returnvalue (Actor|GetActorOfClass "/Game/VERTICAL_SLICE/Blueprints/Luigi_Fake/Luigi_Spline.Luigi_Spline_C"))
  (Variables|Default|SetSplineReference _returnvalue)
  (CallFunction|MoveLuigi))

(event Collision|EventActorBeginOverlap
  (params (OtherActor :type Actor%20Object%20Reference)))

(event EventTick
  (params (DeltaSeconds :type Float%20%28single-precision%29)))

(fn ConstructionScript)